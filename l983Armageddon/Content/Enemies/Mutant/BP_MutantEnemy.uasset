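; Mutant enemy that chases the first-person player once PawnSensing spots them.
; Tick re-issues AI MoveTo while the player is seen, recording SwipeDistance when movement starts.
; Bumping the player subtracts health after a short delay.
; Health is read from the player's MutantHealth variable; at zero, Tick stops movement, disables box collision, flags Dead, then after a delay destroys the actor and increments MutantKills.
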(event `self.ReceiveBeginPlay`
  (bind _asfirst_person_character (cast `/Game/FirstPersonBP/Blueprints/FirstPersonCharacter` (`GameplayStatics.GetPlayerCharacter` 0)))
  (set `self.CharRef` _asfirst_person_character))

(event `self.ReceiveTick`
  (params (DeltaSeconds :type "Float (single-precision)"))
  (bind _charref (`self.CharRef`))
  (if (<= (`/Game/FirstPersonBP/Blueprints/FirstPersonCharacter.MutantHealth` _charref) 0)
    (`PrimitiveComponent.SetCollisionEnabled` (`self.Box`) "NoCollision")
    (set `self.Dead` true)
    (set `self.HasSeen` false)
    (`MovementComponent.StopMovementImmediately` (`self.CharacterMovement`))
    (`KismetSystemLibrary.Delay` 4.6)
    (`self.K2_DestroyActor`)
    (set `/Game/FirstPersonBP/Blueprints/FirstPersonCharacter.MutantKills` (+ (`/Game/FirstPersonBP/Blueprints/FirstPersonCharacter.MutantKills` _charref) 1) _charref)
    (elif (`self.HasSeen`)
      (`|AIMoveTo` self (0.0 0.0 0.0) (`self.CharRef`) 0.0
        (:`then`
          (set `self.SwipeDistance` (`self.GetDistanceTo` (`self.CharRef`))))))))

(event `self.PawnSensing.OnSeePawn`
  (params (Pawn :type "Pawn Object Reference"))
  (cast `/Game/FirstPersonBP/Blueprints/FirstPersonCharacter` Pawn)
  (set `self.HasSeen` true))

(event `self.ReceiveHit`
  (params (MyComp :type "PrimitiveComponent Object Reference") (Other :type "Actor Object Reference") (OtherComp :type "PrimitiveComponent Object Reference") (bSelfMoved :type Boolean) (HitLocation :type "Vector Structure") (HitNormal :type "Vector Structure") (NormalImpulse :type "Vector Structure") (Hit :type "HitResult Structure (by ref)"))
  (bind _charref (`self.CharRef`))
  (cast `/Game/FirstPersonBP/Blueprints/FirstPersonCharacter` Other)
  (`KismetSystemLibrary.Delay` 0.5)
  (set `/Game/FirstPersonBP/Blueprints/FirstPersonCharacter.PlayerHealth` (`KismetMathLibrary.FTrunc` (- (`KismetMathLibrary.Conv_IntToDouble` (`/Game/FirstPersonBP/Blueprints/FirstPersonCharacter.PlayerHealth` _charref)) 20.0)) _charref))

(fn `UserConstructionScript`)